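; BP_RiverRunHUDManager is an actor that puts the River Run HUD on screen and manages mouse cursor mode for the first player controller.
; On BeginPlay it creates WBP_RiverRunHUD, adds it to the viewport and starts with the cursor enabled.
; Tick polls the Tab key to toggle the mode.
; ApplyCursorMode switches between Game and UI and Game Only input, matching cursor visibility to the mode.
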(event `self.ReceiveBeginPlay`
  (set `self.PC` (`GameplayStatics.GetPlayerController` 0))
  (bind _returnvalue (`|CreateWidget` "/Game/RiverRun/UI/WBP_RiverRunHUD.WBP_RiverRunHUD_C" (`self.PC`)))
  (`UserWidget.AddToViewport` _returnvalue 0)
  (set `self.CursorMode` true)
  (`self.ApplyCursorMode`))

(event `self.ReceiveTick`
  (params (DeltaSeconds :type "Float (single-precision)"))
  (if (`PlayerController.WasInputKeyJustPressed` (`self.PC`) "Tab")
    (set `self.CursorMode` (not (`self.CursorMode`)))
    (`self.ApplyCursorMode`)))

(fn `ApplyCursorMode`
  (bind _pc (`self.PC`))
  (bind _cursormode (`self.CursorMode`))
  (if _cursormode
    (`WidgetBlueprintLibrary.SetInputMode_GameAndUIEx` _pc null "DoNotLock" false)
    (else
      (`WidgetBlueprintLibrary.SetInputMode_GameOnly` _pc)))
  (set `PlayerController.bShowMouseCursor` _cursormode _pc))

(fn `UserConstructionScript`)
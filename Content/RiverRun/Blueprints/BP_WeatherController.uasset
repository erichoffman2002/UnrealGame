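; Weather controller for River Run that applies time-of-day presets, cloudiness and rain or snow to the level.
; Setters drive sun rotation, sun/moon forward-shading priority, cloud layer shape and precipitation effects, using actors cached at BeginPlay.
; Rain also changes the river material's roughness, normals and foam.
; Each tick the actor follows the player pawn, stopping precipitation when below the river surface and reapplying weather otherwise.
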(event `self.ReceiveBeginPlay`
  (`self.CacheRefs`)
  (`self.ApplyAll`))

(event `self.ReceiveTick`
  (params (DeltaSeconds :type "Float (single-precision)"))
  (bind _returnvalue (`GameplayStatics.GetPlayerPawn` 0))
  (`/Engine/EditorBlueprintResources/StandardMacros.IsValid` _returnvalue
    (:`Is Valid`
      (`self.K2_SetActorLocation` self (`self.K2_GetActorLocation` _returnvalue) false false)
      (`self.UpdateSubmerged`))))

(fn `ApplyAll`
  (`self.ApplyTime`)
  (`self.ApplyLightPriority`)
  (`self.ApplyClouds`)
  (`self.ApplyWeather`)
  (`self.ApplyWetWater`))

(fn `ApplyClouds`
  (bind _cloudref (`self.CloudRef`))
  (bind _returnvalue (`KismetMathLibrary.FClamp` (`self.Cloudiness`)))
  (`/Engine/EditorBlueprintResources/StandardMacros.IsValid` _cloudref
    (:`Is Valid`
      (bind _asvolumetric_cloud_component (cast `VolumetricCloudComponent` (`self.GetComponentByClass` _cloudref "/Script/Engine.VolumetricCloudComponent")))
      (`VolumetricCloudComponent.SetLayerBottomAltitude` _asvolumetric_cloud_component (- 6.0 (* _returnvalue 3.2)))
      (`VolumetricCloudComponent.SetLayerHeight` _asvolumetric_cloud_component (+ 2.5 (* _returnvalue 9.5))))))

(fn `ApplyLightPriority`
  (bind _sunref (`self.SunRef`))
  (bind _moonref (`self.MoonRef`))
  (bind _returnvalue (== (`self.TimeIndex`) 3))
  (`/Engine/EditorBlueprintResources/StandardMacros.IsValid` _sunref
    (:`Is Valid`
      (bind _asdirectional_light_component (cast `DirectionalLightComponent` (`self.GetComponentByClass` _sunref "/Script/Engine.DirectionalLightComponent")))
      (`DirectionalLightComponent.SetForwardShadingPriority` _asdirectional_light_component (select `bool` _returnvalue :`false` 2 :`true` 0))
      (`/Engine/EditorBlueprintResources/StandardMacros.IsValid` _moonref
        (:`Is Valid`
          (bind _asdirectional_light_component_2 (cast `DirectionalLightComponent` (`self.GetComponentByClass` _moonref "/Script/Engine.DirectionalLightComponent")))
          (`DirectionalLightComponent.SetForwardShadingPriority` _asdirectional_light_component_2 (select `bool` _returnvalue :`false` 0 :`true` 2)))))))

(fn `ApplyTime`
  (bind _timeindex (`self.TimeIndex`))
  (bind _sunref (`self.SunRef`))
  (`/Engine/EditorBlueprintResources/StandardMacros.IsValid` _sunref
    (:`Is Valid`
      (`self.K2_SetActorRotation` _sunref (`KismetMathLibrary.MakeRotator` 0.0 (select `bool` (== _timeindex 0) :`false` (select `bool` (== _timeindex 1) :`false` (select `bool` (== _timeindex 2) :`false` 35.0 :`true` -5.0) :`true` -58.0) :`true` -8.0) (select `bool` (== _timeindex 0) :`false` (select `bool` (== _timeindex 1) :`false` (select `bool` (== _timeindex 2) :`false` -140.0 :`true` -105.0) :`true` 145.0) :`true` 80.0)) false))))

(fn `ApplyWeather`
  (bind _weatherindex (`self.WeatherIndex`))
  (bind _rainfx (`self.RainFX`))
  (bind _snowfx (`self.SnowFX`))
  (if (== _weatherindex 1)
    (`ActorComponent.Activate` _rainfx false)
    (`ActorComponent.Deactivate` _snowfx)
    (elif (== _weatherindex 2)
      (`ActorComponent.Activate` _snowfx false)
      (`ActorComponent.Deactivate` _rainfx)
      (else
        (`ActorComponent.Deactivate` _rainfx)
        (`ActorComponent.Deactivate` _snowfx)))))

(fn `ApplyWetWater`
  (bind _rivercomp (`self.RiverComp`))
  (bind _returnvalue (== (`self.WeatherIndex`) 1))
  (`/Engine/EditorBlueprintResources/StandardMacros.IsValid` _rivercomp
    (:`Is Valid`
      (bind _returnvalue_2 (`WaterBodyComponent.GetWaterMaterialInstance` _rivercomp))
      (`/Engine/EditorBlueprintResources/StandardMacros.IsValid` _returnvalue_2
        (:`Is Valid`
          (`MaterialInstanceDynamic.SetScalarParameterValueByInfo` _returnvalue_2 (make `MaterialParameterInfo` "Water Roughness") (select `bool` _returnvalue :`false` 0.02 :`true` 0.045))
          (`MaterialInstanceDynamic.SetScalarParameterValueByInfo` _returnvalue_2 (make `MaterialParameterInfo` "River Normal Flatness") (select `bool` _returnvalue :`false` 0.5 :`true` 0.1))
          (`MaterialInstanceDynamic.SetScalarParameterValueByInfo` _returnvalue_2 (make `MaterialParameterInfo` "Foam Boost") (select `bool` _returnvalue :`false` 1.0 :`true` 4.0))
          (`MaterialInstanceDynamic.SetScalarParameterValueByInfo` _returnvalue_2 (make `MaterialParameterInfo` "River Foam Scale") (select `bool` _returnvalue :`false` 1536.0 :`true` 260.0))
          (`MaterialInstanceDynamic.SetScalarParameterValueByInfo` _returnvalue_2 (make `MaterialParameterInfo` "FoamContrast") (select `bool` _returnvalue :`false` 1.0 :`true` 0.35))
          (`MaterialInstanceDynamic.SetScalarParameterValueByInfo` _returnvalue_2 (make `MaterialParameterInfo` "Foam Dpeth Min") (select `bool` _returnvalue :`false` 64.0 :`true` 4000.0)))))))

(fn `CacheRefs`
  (bind _outactors (`GameplayStatics.GetAllActorsOfClass` "/Script/Engine.DirectionalLight"))
  (for _array_element _outactors
    (if (`KismetStringLibrary.Contains` (`KismetSystemLibrary.GetDisplayName` _array_element) "Moon")
      (set `self.MoonRef` _array_element)
      (else
        (set `self.SunRef` _array_element))))
  (bind _outactors_2 (`GameplayStatics.GetAllActorsOfClass` "/Script/Engine.ExponentialHeightFog"))
  (for _array_element_2 _outactors_2
    (set `self.FogRef` _array_element_2))
  (bind _outactors_3 (`GameplayStatics.GetAllActorsOfClass` "/Script/Engine.VolumetricCloud"))
  (for _array_element_3 _outactors_3
    (set `self.CloudRef` _array_element_3))
  (bind _outactors_4 (`GameplayStatics.GetAllActorsOfClass` "/Script/Water.WaterBodyRiver"))
  (for _array_element_4 _outactors_4
    (bind _aswater_body (cast `WaterBody` _array_element_4))
    (set `self.RiverComp` (`WaterBody.GetWaterBodyComponent` _aswater_body))))

(fn `SetCloudsTo`
  (params (NewClouds :type "Float (double-precision)"))
  (set `self.Cloudiness` NewClouds)
  (`self.ApplyClouds`))

(fn `SetTimeTo`
  (params (NewTime :type Integer))
  (set `self.TimeIndex` NewTime)
  (`self.ApplyAll`))

(fn `SetWeatherTo`
  (params (NewWeather :type Integer))
  (set `self.WeatherIndex` NewWeather)
  (`self.ApplyWeather`)
  (`self.ApplyWetWater`))

(fn `UpdateSubmerged`
  (bind _rivercomp (`self.RiverComp`))
  (bind _returnvalue (`self.K2_GetActorLocation` self))
  (bind (_outwatersurfacelocation _outwatersurfacenormal _outwatervelocity _outwaterdepth _returnvalue_2) (`WaterBodyComponent.GetWaterSurfaceInfoAtLocation` _rivercomp _returnvalue false))
  (bind _returnvalue_3 (and _returnvalue_2 (> (- (.z _outwatersurfacelocation) (.z _returnvalue)) 0.0)))
  (`/Engine/EditorBlueprintResources/StandardMacros.IsValid` _rivercomp
    (:`Is Valid`
      (set `self.bSubmerged` _returnvalue_3)
      (if _returnvalue_3
        (`ActorComponent.Deactivate` (`self.RainFX`))
        (`ActorComponent.Deactivate` (`self.SnowFX`))
        (else
          (`self.ApplyWeather`))))))

(fn `UserConstructionScript`)
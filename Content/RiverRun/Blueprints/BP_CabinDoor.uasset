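; BP_CabinDoor is a clickable cabin door that swings on a Hinge component.
; Each click flips Open and sets the target yaw: OpenAngle when Open becomes false, zero when it becomes true.
; Tick eases CurrentYaw toward the target with FInterpTo, then applies a second interpolation step from that value as the hinge's relative yaw.
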(event `self.ReceiveActorOnClicked`
  (params (ButtonPressed :type "Key Structure"))
  (bind _returnvalue (not (`self.bOpen`)))
  (set `self.bOpen` _returnvalue)
  (if _returnvalue
    (set `self.TargetYaw` (`self.OpenAngle`))
    (else
      (set `self.TargetYaw` 0.0))))

(event `self.ReceiveTick`
  (params (DeltaSeconds :type "Float (single-precision)"))
  (bind _returnvalue (`KismetMathLibrary.FInterpTo` (`self.CurrentYaw`) (`self.TargetYaw`) DeltaSeconds 3.5))
  (set `self.CurrentYaw` _returnvalue)
  (`SceneComponent.K2_SetRelativeRotation` (`self.Hinge`) (`KismetMathLibrary.MakeRotator` 0.0 0.0 _returnvalue) false false))

(fn `UserConstructionScript`)
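; BP_Campfire is a clickable campfire actor that the player can light and put out.
; On BeginPlay it makes ClickBox a query-only volume that blocks only the WorldStatic channel.
; Clicking calls ToggleFire, which flips the Lit flag and switches the Flames effect and Light visibility to match.
; Hovering the cursor over it shows the Hint component, which hides again when the cursor leaves.
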(event `self.ReceiveBeginPlay`
  (bind _clickbox (`self.ClickBox`))
  (`PrimitiveComponent.SetCollisionEnabled` _clickbox "QueryOnly")
  (`PrimitiveComponent.SetCollisionResponseToAllChannels` _clickbox "ECR_Ignore")
  (`PrimitiveComponent.SetCollisionResponseToChannel` _clickbox "ECC_WorldStatic" "ECR_Block"))

(event `self.ReceiveActorOnClicked`
  (params (ButtonPressed :type "Key Structure"))
  (`self.ToggleFire`))

(event `self.ReceiveActorBeginCursorOver`
  (`SceneComponent.SetVisibility` (`self.Hint`) true false))

(event `self.ReceiveActorEndCursorOver`
  (`SceneComponent.SetVisibility` (`self.Hint`) false false))

(fn `ToggleFire`
  (bind _flames (`self.Flames`))
  (bind _light (`self.Light`))
  (if (`self.bLit`)
    (set `self.bLit` false)
    (`ActorComponent.Deactivate` _flames)
    (`SceneComponent.SetVisibility` _light false false)
    (else
      (set `self.bLit` true)
      (`ActorComponent.Activate` _flames true)
      (`SceneComponent.SetVisibility` _light true false))))

(fn `UserConstructionScript`)
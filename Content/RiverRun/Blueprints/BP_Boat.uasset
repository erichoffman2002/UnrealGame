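; Physics-driven boat that rides the river's current, catches fire when another actor overlaps it, then sinks.
; Each tick it applies depth-scaled buoyancy at four hull corners, plus drag toward the water velocity and a layered-sine bob, using surface queries on a WaterBodyRiver.
; Ignition starts the fire effect and a burn timer that zeroes buoyancy.
; Submersion douses the flames, and physics switches off once the sunken hull is deep and slow.
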(event `self.ReceiveBeginPlay`
  (bind _outactors (`GameplayStatics.GetAllActorsOfClass` "/Script/Water.WaterBodyRiver"))
  (for _array_element _outactors
    (bind _aswater_body (cast `WaterBody` _array_element))
    (set `self.RiverComp` (`WaterBody.GetWaterBodyComponent` _aswater_body))))

(event `self.ReceiveActorBeginOverlap`
  (params (OtherActor :type "Actor Object Reference"))
  (`self.Ignite`))

(event `self.ReceiveTick`
  (params (DeltaSeconds :type "Float (single-precision)"))
  (`self.FloatAt` (`KismetMathLibrary.MakeVector` 150.0 55.0 -30.0))
  (`self.FloatAt` (`KismetMathLibrary.MakeVector` 150.0 -55.0 -30.0))
  (`self.FloatAt` (`KismetMathLibrary.MakeVector` -150.0 55.0 -30.0))
  (`self.FloatAt` (`KismetMathLibrary.MakeVector` -150.0 -55.0 -30.0))
  (`self.ApplyCurrent`)
  (`self.UpdateFire`)
  (`self.UpdateRest`))

(fn `ApplyCurrent`
  (bind _returnvalue (`self.K2_GetActorLocation`))
  (bind _returnvalue_2 (`KismetSystemLibrary.GetGameTimeInSeconds`))
  (bind _rivercomp (`self.RiverComp`))
  (bind _hull (`self.Hull`))
  (bind (_outwatersurfacelocation _outwatersurfacenormal _outwatervelocity _outwaterdepth _returnvalue_3) (`WaterBodyComponent.GetWaterSurfaceInfoAtLocation` _rivercomp _returnvalue false))
  (bind _returnvalue_4 (- (.z _outwatersurfacelocation) (.z _returnvalue)))
  (`/Engine/EditorBlueprintResources/StandardMacros.IsValid` _rivercomp
    (:`Is Valid`
      (if (and (and _returnvalue_3 (not (`self.bSunk`))) (and (> _returnvalue_4 -80.0) (< _returnvalue_4 (`self.DragCutoffDepth`))))
        (bind _returnvalue_5 (`PrimitiveComponent.GetPhysicsLinearVelocity` _hull "None"))
        (`PrimitiveComponent.AddForce` _hull (* (- _outwatervelocity _returnvalue_5) (`self.DragStrength`)) "None" false)
        (`PrimitiveComponent.AddForce` _hull (`KismetMathLibrary.MakeVector` 0.0 0.0 (* (+ (`KismetMathLibrary.Sin` (* _returnvalue_2 1.7)) (* (`KismetMathLibrary.Sin` (* _returnvalue_2 1.1)) 0.5)) (`self.BobStrength`))) "None" false)))))

(fn `FloatAt`
  (params (Offset :type "Vector Structure"))
  (bind _rivercomp (`self.RiverComp`))
  (bind _returnvalue (+ (`self.K2_GetActorLocation`) (`KismetMathLibrary.GreaterGreater_VectorRotator` (`KismetMathLibrary.Conv_RotatorToVector` (`self.K2_GetActorRotation`)) (`KismetMathLibrary.Conv_VectorToRotator` Offset))))
  (bind (_outwatersurfacelocation _outwatersurfacenormal _outwatervelocity _outwaterdepth _returnvalue_2) (`WaterBodyComponent.GetWaterSurfaceInfoAtLocation` _rivercomp _returnvalue false))
  (bind _returnvalue_3 (- (.z _outwatersurfacelocation) (.z _returnvalue)))
  (`/Engine/EditorBlueprintResources/StandardMacros.IsValid` _rivercomp
    (:`Is Valid`
      (if (and _returnvalue_2 (> _returnvalue_3 0.0))
        (`PrimitiveComponent.AddForceAtLocation` (`self.Hull`) (`KismetMathLibrary.MakeVector` 0.0 0.0 (* (`KismetMathLibrary.FClamp` _returnvalue_3 0.0 120.0) (`self.FloatStrength`))) _returnvalue "None")))))

(fn `Ignite`
  (if (not (`self.bIgnited`))
    (set `self.bIgnited` true)
    (set `self.bFireLit` true)
    (`ActorComponent.Activate` (`self.FireFX`) true)
    (`KismetSystemLibrary.K2_SetTimer` self "Sink" (`self.BurnSeconds`))))

(fn `Sink`
  (set `self.FloatStrength` 0.0))

(fn `UpdateFire`
  (bind _returnvalue (`self.K2_GetActorLocation`))
  (bind _rivercomp (`self.RiverComp`))
  (bind (_outwatersurfacelocation _outwatersurfacenormal _outwatervelocity _outwaterdepth _returnvalue_2) (`WaterBodyComponent.GetWaterSurfaceInfoAtLocation` _rivercomp _returnvalue false))
  (`/Engine/EditorBlueprintResources/StandardMacros.IsValid` _rivercomp
    (:`Is Valid`
      (if (and (`self.bFireLit`) (and _returnvalue_2 (> (- (.z _outwatersurfacelocation) (.z _returnvalue)) (`self.DouseDepth`))))
        (set `self.bFireLit` false)
        (`ActorComponent.Deactivate` (`self.FireFX`))))))

(fn `UpdateRest`
  (bind _returnvalue (`self.K2_GetActorLocation`))
  (bind _rivercomp (`self.RiverComp`))
  (bind _hull (`self.Hull`))
  (bind (_outwatersurfacelocation _outwatersurfacenormal _outwatervelocity _outwaterdepth _returnvalue_2) (`WaterBodyComponent.GetWaterSurfaceInfoAtLocation` _rivercomp _returnvalue false))
  (`/Engine/EditorBlueprintResources/StandardMacros.IsValid` _rivercomp
    (:`Is Valid`
      (bind _returnvalue_3 (`PrimitiveComponent.GetPhysicsLinearVelocity` _hull "None"))
      (if (and (and (not (`self.bSunk`)) (`self.bIgnited`)) (and (and _returnvalue_2 (> (- (.z _outwatersurfacelocation) (.z _returnvalue)) (`self.DragCutoffDepth`))) (< (`KismetMathLibrary.VSize` _returnvalue_3) (`self.RestSpeed`))))
        (set `self.bSunk` true)
        (`PrimitiveComponent.SetSimulatePhysics` _hull false)))))

(fn `UserConstructionScript`)